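; BP_LightProjectionResolver converts a screen-space light center UV into a world position on a vertical plane of constant Y.
; ResolveLightProjection scales the UV by viewport size, deprojects it through player 0's controller and solves the ray-plane intersection at ProjectionPlaneY, flagging rays nearly parallel to the plane as invalid.
; Tick re-resolves the stored UV each frame and, when valid, draws debug spheres at a fixed point and near the projected position.
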(event `self.ReceiveTick`
  (params (DeltaSeconds :type "Float (single-precision)"))
  (bind (_outlightworldposition _outhasvalidprojection) (`self.ResolveLightProjection` (`self.LightCenterUV`)))
  (bind _output_get (set `self.HasValidProjection` _outhasvalidprojection))
  (if _output_get
    (bind _output_get_2 (set `self.LightWorldPosition` _outlightworldposition))
    (`KismetSystemLibrary.DrawDebugSphere` (0.0 -20.0 200.0) 80.0 100 (struct :`G` 1.0 :`B` 0.248524 :`A` 1.0) 0.05 5.0)
    (`KismetSystemLibrary.DrawDebugSphere` (+ _output_get_2 (0.0 -50.0 0.0)) 120.0 10 (struct :`R` 1.0 :`G` 0.669542 :`B` 0.014306 :`A` 1.0) 0.03 2.0)))

(fn `ResolveLightProjection`
  (params (InLightCenterUV :type "Vector2D Structure"))
  (returns (OutLightWorldPosition :type "Vector Structure") (OutHasValidProjection :type Boolean))
  (bind _returnvalue (`GameplayStatics.GetPlayerController` 0))
  (bind (_lightcenteruv_x _lightcenteruv_y) (`KismetMathLibrary.BreakVector2D` (`self.LightCenterUV`)))
  (bind (_sizex _sizey) (`PlayerController.GetViewportSize` _returnvalue))
  (bind (_worldlocation _worlddirection) (`PlayerController.DeprojectScreenPositionToWorld` _returnvalue (* _sizex _lightcenteruv_x) (* _sizey _lightcenteruv_y)))
  (bind _y (.y _worlddirection))
  ; Input Screen UV
  (set `self.LightCenterUV` InLightCenterUV)
  ; T value: determines the distance along the ray to reach the target plane
  (if (> (`KismetMathLibrary.Abs` _y) 0.001)
    (bind _output_get (set `self.HasValidProjection` true))
    ; Calculate the world position
    (bind _output_get_2 (set `self.LightWorldPosition` (+ (* _worlddirection (/ (- (`self.ProjectionPlaneY`) (.y _worldlocation)) _y)) _worldlocation)))
    (return _output_get_2 _output_get)
    (else
      (bind _output_get_3 (set `self.HasValidProjection` false))
      (return (`self.LightWorldPosition`) _output_get_3))))

(fn `UserConstructionScript`)