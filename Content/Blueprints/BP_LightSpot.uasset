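; BP_LightSpot holds the state of a projected light spot and publishes it to the MPC_Light material parameter collection.
; UpdateLightSpot receives center UV, world position and projection validity from its caller; the actor has no active events of its own.
; Valid projections draw a debug sphere and write position, radius, feather, intensity and focus to the collection.
; Invalid ones only zero HasValidProjection, with no collection assigned; the valid branch never sets that parameter.
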(fn `UpdateLightSpot`
  (params (InLightCenterUV :type "Vector2D Structure") (InLightWorldPosition :type "Vector Structure") (InHasValidProjection :type Boolean))
  (bind (_lightcenteruv_x _lightcenteruv_y) (`KismetMathLibrary.BreakVector2D` (`self.LightCenterUV`)))
  (set `self.LightCenterUV` InLightCenterUV)
  (set `self.LightWorldPosition` InLightWorldPosition)
  (set `self.HasValidProjection` InHasValidProjection)
  ; 光源状态中心
  (if (`self.HasValidProjection`)
    (`KismetSystemLibrary.DrawDebugSphere` (`self.LightWorldPosition`) (`self.LightRadius`) 12 (struct :`G` 0.168022 :`B` 1.0 :`A` 1.0))
    (`KismetMaterialLibrary.SetVectorParameterValue` "/Game/Material/MPC_Light.MPC_Light" "Light Center UV" (`KismetMathLibrary.Conv_VectorToLinearColor` (`KismetMathLibrary.MakeVector` _lightcenteruv_x _lightcenteruv_y)))
    (`KismetMaterialLibrary.SetVectorParameterValue` "/Game/Material/MPC_Light.MPC_Light" "Light World Position" (`KismetMathLibrary.Conv_VectorToLinearColor` (`self.LightWorldPosition`)))
    (`KismetMaterialLibrary.SetScalarParameterValue` "/Game/Material/MPC_Light.MPC_Light" "Focus Amount" (`self.FocusAmount`))
    (`KismetMaterialLibrary.SetScalarParameterValue` "/Game/Material/MPC_Light.MPC_Light" "Light Feather" (`self.LightFeather`))
    (`KismetMaterialLibrary.SetScalarParameterValue` "/Game/Material/MPC_Light.MPC_Light" "Light Intensity" (`self.LightIntensity`))
    (`KismetMaterialLibrary.SetScalarParameterValue` "/Game/Material/MPC_Light.MPC_Light" "Light Radius" (`self.LightRadius`))
    (else
      (`KismetMaterialLibrary.SetScalarParameterValue` null "HasValidProjection"))))

(fn `UserConstructionScript`)