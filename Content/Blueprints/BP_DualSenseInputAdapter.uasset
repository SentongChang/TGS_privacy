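; Input adapter actor that steers a projected light spot's center in UV space from Enhanced Input look values (IMC_MouseLook, despite the DualSense name).
; Tick integrates input into a clamped target UV and interpolates the current center toward it; IA_BackToCenter snaps both to screen middle.
; The level's BP_LightProjectionResolver converts that UV to a world position and validity flag, which are passed to LightSpot.
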(event `self.ReceiveBeginPlay`
  ; Gyro_Start & Recorded the new center.
  (`|ExecutionSequence`
    (:`then_0`
      ;;[0.15 0.06554 0.06976 0.5] BP_LightProjection Resolver
      (bind _returnvalue (`GameplayStatics.GetActorOfClass` "/Game/Blueprints/BP_LightProjectionResolver.BP_LightProjectionResolver_C"))
      (set `self.LightProjectionResolver` _returnvalue))
    (:`then_1`
      (`self.EnableInput` (`GameplayStatics.GetPlayerController` 0))
      (`EnhancedInputSubsystemInterface.AddMappingContext` (pcsubsystem `EnhancedInputLocalPlayerSubsystem` (`GameplayStatics.GetPlayerController` 0)) "/SST/SST/Input/IMC_MouseLook.IMC_MouseLook" 0 (struct)))
    (:`then_2`
      ; Start & Get data
      (set `self.TargetLightCenterUV` (0.5 0.5) :!label _label)
      (set `self.LightCenterUV` (0.5 0.5)))))

(event `EnhancedInput|/SST/SST/Input/Actions/IA_BackToCenter`
  (params (ActionValue :type Boolean) (ElapsedSeconds :type "Float (double-precision)") (TriggeredSeconds :type "Float (double-precision)") (InputAction :type "InputAction Object Reference" :default "/SST/SST/Input/Actions/IA_BackToCenter.IA_BackToCenter"))
  ; Start & Get data
  (:`Triggered`
    (goto _label)))

(event `EnhancedInput|/Game/Input/Actions/IA_MouseLook`
  (params (ActionValue :type "Vector2D Structure") (ElapsedSeconds :type "Float (double-precision)") (TriggeredSeconds :type "Float (double-precision)") (InputAction :type "InputAction Object Reference" :default "/Game/Input/Actions/IA_MouseLook.IA_MouseLook"))
  ; Start & Get data
  (:`Triggered`
    (bind _output_get (set `self.AimStickInput X` ActionValue_X))
    (bind _output_get_2 (set `self.AimStickInput Y` ActionValue_Y))
    (`KismetSystemLibrary.PrintString` (`KismetStringLibrary.Concat_StrStr` (`KismetStringLibrary.Concat_StrStr` "X" (`KismetStringLibrary.Conv_DoubleToString` _output_get)) (`KismetStringLibrary.Concat_StrStr` "Y" (`KismetStringLibrary.Conv_DoubleToString` _output_get_2))))))

(event `self.ReceiveTick`
  (params (DeltaSeconds :type "Float (single-precision)"))
  (bind _lightprojectionresolver (`self.LightProjectionResolver`))
  (bind _aimspeed (`self.AimSpeed`))
  (bind (_targetlightcenteruv_x _targetlightcenteruv_y) (`KismetMathLibrary.BreakVector2D` (`self.TargetLightCenterUV`)))
  ; UV Maping
  (bind _output_get (set `self.TargetX` (`KismetMathLibrary.FClamp` (+ (* (* (`self.AimStickInput X`) _aimspeed) DeltaSeconds) _targetlightcenteruv_x) 0.08 0.92)))
  (bind _output_get_2 (set `self.TargetY` (`KismetMathLibrary.FClamp` (+ (* (* (`self.AimStickInput Y`) _aimspeed) DeltaSeconds) _targetlightcenteruv_y) 0.08 0.92)))
  (set `self.TargetLightCenterUV` (`KismetMathLibrary.MakeVector2D` _output_get _output_get_2))
  (bind _output_get_3 (set `self.LightCenterUV` (`KismetMathLibrary.Vector2DInterpTo` (`self.LightCenterUV`) (`self.TargetLightCenterUV`) DeltaSeconds (`self.Interp Speed`))))
  ;[0.15 0.09636 0.1366 0.5] BP_LightProjection Resolver
  (`/Engine/EditorBlueprintResources/StandardMacros.IsValid` _lightprojectionresolver
    (:`Is Valid`
      (bind (_outlightworldposition _outhasvalidprojection) (`/Game/Blueprints/BP_LightProjectionResolver.ResolveLightProjection` _lightprojectionresolver _output_get_3))
      (bind _output_get_4 (set `self.Out Light World Position` _outlightworldposition))
      (set `self.Out Has Valid Projection` _outhasvalidprojection)
      (`/Engine/EditorBlueprintResources/StandardMacros.IsValid` null
        (:`Is Valid`
          (`/Game/Blueprints/BP_LightSpot.UpdateLightSpot` (`self.LightSpot`) (`self.LightCenterUV`) (`self.Out Light World Position`) (`self.Out Has Valid Projection`)))))))

(fn `UserConstructionScript`)